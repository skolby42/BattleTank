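; Tank pawn Blueprint that handles input for aiming, firing and track-based movement.
; On BeginPlay it hands barrel, turret and both tracks to the TankAiming and TankMovement components, then links itself to its HealthBar widget.
; Aim axes rotate the azimuth gimbal and spring arm, while fire and movement inputs forward to those components.
; The construction script sets the projectile class as a hot reload workaround.
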(event `self.ReceiveBeginPlay`
  (`TankAimingComponent.Initialize` (`self.TankAiming`) (`self.Barrel`) (`self.Turret`))
  (`TankMovementComponent.Initialize` (`self.TankMovement`) (`self.LeftTrack`) (`self.RightTrack`))
  (`self.InitializeHealthBarWidget`))

(event `InputAxis|AimAzimuth`
  (params (AxisValue :type "Float (single-precision)"))
  ;[1 1 1] Ballistics Input binding
  (`SceneComponent.K2_AddLocalRotation` (`self.AzimuthGimbal`) (`KismetMathLibrary.MakeRotator` 0.0 0.0 AxisValue) false false))

(event `InputAxis|AimElevation`
  (params (AxisValue :type "Float (single-precision)"))
  ;[1 1 1] Ballistics Input binding
  (`SceneComponent.K2_AddLocalRotation` (`self.SpringArm`) (`KismetMathLibrary.MakeRotator` 0.0 AxisValue) false false))

(event `InputAction|Fire`
  (params (Key :type "Key Structure"))
  ;[1 1 1] Ballistics Input binding
  (:`Pressed`
    (`TankAimingComponent.Fire` (`self.TankAiming`))))

(event `InputAxis|Move Forward`
  (params (AxisValue :type "Float (single-precision)"))
  ;[1 1 1] Movement input binding
  (`TankMovementComponent.IntendMoveForward` (`self.TankMovement`) AxisValue))

(event `InputAxis|Turn Right`
  (params (AxisValue :type "Float (single-precision)"))
  ;[1 1 1] Movement input binding
  (`TankMovementComponent.IntendTurnRight` (`self.TankMovement`) AxisValue))

(fn `InitializeHealthBarWidget`
  (bind _ashealth_bar (cast `/Game/UI/HealthBar` (`WidgetComponent.GetUserWidgetObject` (`self.HealthBar`)))
    (:`then`
      (set `/Game/UI/HealthBar.Tank` self _ashealth_bar))
    (:`CastFailed`
      _))
  (return))

(fn `UserConstructionScript`
  ;[1 1 1] Workaround for hot reload bug
  (set `TankAimingComponent.ProjectileBlueprint` "/Game/Assets/Projectile/Projectile_BP.Projectile_BP_C" (`self.TankAiming`)))